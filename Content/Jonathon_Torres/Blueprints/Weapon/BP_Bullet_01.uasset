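; BP_Bullet_01 is a bullet actor that damages enemies on overlap and then destroys itself.
; Three hit boxes each cast the overlapping actor to one class: Enemy, EnemyPatrol or BP_Ai_Guard.
; A successful cast directly subtracts a fixed amount from that enemy's HealthPercentage, with EnemyPatrol losing the most.
; Guard hits also play a hurt sound at the world origin, and failed casts leave the bullet intact.
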(event `self.HitBox.OnComponentBeginOverlap`
  (params (OverlappedComponent :type "PrimitiveComponent Object Reference") (OtherActor :type "Actor Object Reference") (OtherComp :type "PrimitiveComponent Object Reference") (OtherBodyIndex :type Integer) (bFromSweep :type Boolean) (SweepResult :type "HitResult Structure (by ref)"))
  (bind _asenemy (cast `/Game/Jonathon_Torres/Blueprints/Enemy/Enemy` OtherActor))
  (set `/Game/Jonathon_Torres/Blueprints/Enemy/Enemy.Health Percentage` (- (`/Game/Jonathon_Torres/Blueprints/Enemy/Enemy.Health Percentage` _asenemy) 0.1) _asenemy)
  (`self.K2_DestroyActor`))

(event `self.HitBox2.OnComponentBeginOverlap`
  (params (OverlappedComponent :type "PrimitiveComponent Object Reference") (OtherActor :type "Actor Object Reference") (OtherComp :type "PrimitiveComponent Object Reference") (OtherBodyIndex :type Integer) (bFromSweep :type Boolean) (SweepResult :type "HitResult Structure (by ref)"))
  (bind _asenemy_patrol (cast `/Game/Jonathon_Torres/Blueprints/EnemyPatrol/EnemyPatrol` OtherActor))
  (set `/Game/Jonathon_Torres/Blueprints/EnemyPatrol/EnemyPatrol.Health Percentage` (- (`/Game/Jonathon_Torres/Blueprints/EnemyPatrol/EnemyPatrol.Health Percentage` _asenemy_patrol) 0.3) _asenemy_patrol)
  (`self.K2_DestroyActor`))

(event `self.HitBox3.OnComponentBeginOverlap`
  (params (OverlappedComponent :type "PrimitiveComponent Object Reference") (OtherActor :type "Actor Object Reference") (OtherComp :type "PrimitiveComponent Object Reference") (OtherBodyIndex :type Integer) (bFromSweep :type Boolean) (SweepResult :type "HitResult Structure (by ref)"))
  (bind _asbp_ai_guard (cast `/Game/AI/WithBehaviourTree/Guard/BP_Ai_Guard` OtherActor))
  (`GameplayStatics.PlaySoundAtLocation` "/Game/Jonathon_Torres/Blueprints/Sound_Effects/Oof_Better.Oof_Better" (0.0 0.0 0.0) (struct) 1.0 1.0 0.0 null null _asbp_ai_guard)
  (set `/Game/AI/WithBehaviourTree/Guard/BP_Ai_Guard.Health Percentage` (- (`/Game/AI/WithBehaviourTree/Guard/BP_Ai_Guard.Health Percentage` _asbp_ai_guard) 0.1) _asbp_ai_guard)
  (`self.K2_DestroyActor`))

(fn `UserConstructionScript`)