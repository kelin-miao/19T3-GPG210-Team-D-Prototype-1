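; Enemy actor that the player can destroy for points and that kills the player on contact.
; TakeDamage lowers clamped Health and updates HealthPercentage, which Tick polls to destroy the enemy and add TargetScore through ThirdPersonGameMode.
; A Hitbox overlap with the Player writes its health percentage, then immediately destroys player pawn 0.
; Health bar widget binding and hit-delay logic remain only as disconnected, archived nodes.
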(event `self.ReceiveBeginPlay`
  ;[1 1 1] HealthBar
)

(event `self.ReceiveTick`
  (params (DeltaSeconds :type "Float (single-precision)"))
  ;[1 0.2083 0.2083] WhenTakingDamage
  (`|ExecutionSequence`
    (:`then_1`
      (if (<= (`self.Health Percentage`) 0.0)
        (`self.K2_DestroyActor`)
        (bind _asthird_person_game_mode (cast `/Game/Jonathon_Torres/Blueprints/ThirdPersonGameMode` (`GameplayStatics.GetGameMode`)))
        (`/Game/Jonathon_Torres/Blueprints/ThirdPersonGameMode.AddTargetPoints` _asthird_person_game_mode (`self.Target Score`))))))

(event `self.Hitbox.OnComponentBeginOverlap`
  (params (OverlappedComponent :type "PrimitiveComponent Object Reference") (OtherActor :type "Actor Object Reference") (OtherComp :type "PrimitiveComponent Object Reference") (OtherBodyIndex :type Integer) (bFromSweep :type Boolean) (SweepResult :type "HitResult Structure (by ref)"))
  ;[1 1 1] The Player dies instantly
  (bind _asplayer (cast `/Game/Jonathon_Torres/Blueprints/Player` OtherActor))
  (set `/Game/Jonathon_Torres/Blueprints/Player.PlayerHealthPercentage` (- (`/Game/Jonathon_Torres/Blueprints/Player.PlayerHealth` _asplayer) 0.1) _asplayer)
  (`self.K2_DestroyActor` (`GameplayStatics.GetPlayerPawn` 0)))

(fn `TakeDamage`
  (params (Damage :type "Float (double-precision)"))
  (bind _output_get (set `self.Health` (`KismetMathLibrary.FClamp` (- (`self.Health`) Damage) 0.0 100.0)))
  (set `self.Health Percentage` (/ _output_get 100.0)))

(fn `UserConstructionScript`)