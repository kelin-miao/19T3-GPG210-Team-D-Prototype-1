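; BP_Enemy is an enemy actor that hurts the player on contact and awards points when killed.
; BeginPlay links it to its health bar widget, and TakeDamage clamps Health and updates HealthPercentage.
; Tick polls that percentage, destroying the actor at zero and adding TargetScore through ThirdPersonGameMode.
; Hitbox overlap damages BP_Player and runs a timeline that toggles HitDelay, which no live logic checks.
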(event `self.ReceiveBeginPlay`
  ;[1 1 1] HealthBar
  (bind _aswb_enemy_health_ui (cast `/Game/Jonathon_Torres/Blueprints/Widgets/WB_EnemyHealthUI` (`WidgetComponent.GetUserWidgetObject` (`self.EnemyHealthUI`))))
  (set `/Game/Jonathon_Torres/Blueprints/Widgets/WB_EnemyHealthUI.Enemy` self _aswb_enemy_health_ui))

(event `self.ReceiveTick`
  (params (DeltaSeconds :type "Float (single-precision)"))
  ;[1 0.2083 0.2083] WhenTakingDamage
  (`|ExecutionSequence`
    (:`then_1`
      (if (<= (`self.Health Percentage`) 0.0)
        (`self.K2_DestroyActor`)
        (bind _asthird_person_game_mode (cast `/Game/Jonathon_Torres/Blueprints/ThirdPersonGameMode` (`GameplayStatics.GetGameMode`)))
        (`/Game/Jonathon_Torres/Blueprints/ThirdPersonGameMode.AddTargetPoints` _asthird_person_game_mode (`self.Target Score`))))))

(event `self.Hitbox.OnComponentBeginOverlap`
  (params (OverlappedComponent :type "PrimitiveComponent Object Reference") (OtherActor :type "Actor Object Reference") (OtherComp :type "PrimitiveComponent Object Reference") (OtherBodyIndex :type Integer) (bFromSweep :type Boolean) (SweepResult :type "HitResult Structure (by ref)"))
  ;[1 1 1] The Player dies instantly
  (bind _asbp_player (cast `/Game/Jonathon_Torres/Blueprints/BP_Player` OtherActor))
  (`/Game/Jonathon_Torres/Blueprints/BP_Player.PlayerTakeDamage` _asbp_player 2.5)
  (set `self.HitDelay` true)
  (`Timeline|Timeline_0` :!via `PlayFromStart`
    (:`Finished`
      (set `self.HitDelay` false))))

(fn `TakeDamage`
  (params (Damage :type "Float (double-precision)"))
  (bind _output_get (set `self.Health` (`KismetMathLibrary.FClamp` (- (`self.Health`) Damage) 0.0 100.0)))
  (set `self.Health Percentage` (/ _output_get 100.0)))

(fn `UserConstructionScript`)