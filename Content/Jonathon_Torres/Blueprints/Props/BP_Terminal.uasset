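; Terminal prop that shows a WB_Terminal mission widget on the game mode's HUD canvas when BP_Player enters its sphere.
; Overlap begin creates and anchors the widget, or removes it if one already exists; overlap end jumps into that same removal path, which also creates an unused widget.
; A side branch tries to add QuestLog's CrossedOUt element to the canvas, but only runs when QuestLog is invalid.
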(event `self.Sphere.OnComponentBeginOverlap`
  (params (OverlappedComponent :type "PrimitiveComponent Object Reference") (OtherActor :type "Actor Object Reference") (OtherComp :type "PrimitiveComponent Object Reference") (OtherBodyIndex :type Integer) (bFromSweep :type Boolean) (SweepResult :type "HitResult Structure (by ref)"))
  (cast `/Game/Jonathon_Torres/Blueprints/BP_Player` OtherActor)
  (`KismetSystemLibrary.PrintString` "Hello")
  (bind _terminalmission (`self.TerminalMission`)
    (:`then`
      (`|CreateWidget` "/Game/Jonathon_Torres/Blueprints/Widgets/WB_Terminal.WB_Terminal_C" :!label _label)
      (`Widget.RemoveFromParent` _terminalmission)
      (set `self.TerminalMission` null))
    (:`else`
      (`|ExecutionSequence`
        (:`then_0`
          (bind _questlog (`self.QuestLog`)
            (:`then`)
            (:`else`
              (set `self.QuestLog` null)
              (bind _asthird_person_game_mode (cast `/Game/Jonathon_Torres/Blueprints/ThirdPersonGameMode` (`GameplayStatics.GetGameMode`)))
              (bind _returnvalue (`CanvasPanel.AddChildToCanvas` (`/Game/Jonathon_Torres/Blueprints/ThirdPersonGameMode.HUD_Canvas` _asthird_person_game_mode) (`/Game/Jonathon_Torres/Blueprints/Widgets/WB_QuestLogUI.CrossedOUt` _questlog)))
              (`CanvasPanelSlot.SetAnchors` _returnvalue (make `Anchors` (0.0 0.0) (1.0 1.0))))))
        (:`then_1`
          (bind _returnvalue_2 (`|CreateWidget` "/Game/Jonathon_Torres/Blueprints/Widgets/WB_Terminal.WB_Terminal_C"))
          (set `self.TerminalMission` _returnvalue_2)
          (bind _asthird_person_game_mode_2 (cast `/Game/Jonathon_Torres/Blueprints/ThirdPersonGameMode` (`GameplayStatics.GetGameMode`)))
          (bind _returnvalue_3 (`CanvasPanel.AddChildToCanvas` (`/Game/Jonathon_Torres/Blueprints/ThirdPersonGameMode.HUD_Canvas` _asthird_person_game_mode_2) (`self.TerminalMission`)))
          (`CanvasPanelSlot.SetAnchors` _returnvalue_3 (make `Anchors` (1.0 1.0))))))))

(event `self.Sphere.OnComponentEndOverlap`
  (params (OverlappedComponent :type "PrimitiveComponent Object Reference") (OtherActor :type "Actor Object Reference") (OtherComp :type "PrimitiveComponent Object Reference") (OtherBodyIndex :type Integer))
  (cast `/Game/Jonathon_Torres/Blueprints/BP_Player` OtherActor)
  (goto _label))

(fn `UserConstructionScript`)