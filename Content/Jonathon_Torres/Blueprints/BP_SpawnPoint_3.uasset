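; BP_SpawnPoint_3 is an enemy spawn point that creates AI pawns with behavior trees when its Random event fires.
; Random calls SpawnEnemy3, then spawns an extra shooting enemy at the Arrow component.
; SpawnEnemy3 spawns a guard or shooter at the actor's transform, with the clamped roll heavily favoring shooters.
; The under-100 check measures a single-element array, so it never limits spawning.
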(event `Random`
  ;[1 1 1] SpawnEnemybyDifficulty
  (if (< (`KismetArrayLibrary.Array_Length` (`|MakeArray` (stale _returnvalue) :!type "Actor Object Reference")) 100)
    (`self.SpawnEnemy3`)
    (bind _returnvalue (`AIBlueprintHelperLibrary.SpawnAIFromClass` "/Game/AI/Testing/ShootingAi/BP_ShootingEnemy.BP_ShootingEnemy_C" "/Game/AI/Testing/ShootingAi/BT_ShootingEnemy.BT_ShootingEnemy" (`SceneComponent.K2_GetComponentLocation` (`self.Arrow`))))))

(fn `SpawnEnemy3`
  (bind (_returnvalue_location _returnvalue_rotation) (`KismetMathLibrary.BreakTransform` (`self.GetTransform`)))
  (switch `int` (`KismetMathLibrary.Clamp` (`KismetMathLibrary.RandomInteger` 20) 1 2)
    (:`1`
      (`AIBlueprintHelperLibrary.SpawnAIFromClass` "/Game/AI/Testing/Guard/BP_Ai_Guard.BP_Ai_Guard_C" "/Game/AI/Testing/Guard/BT_Guard.BT_Guard" _returnvalue_location _returnvalue_rotation))
    (:`2`
      (`AIBlueprintHelperLibrary.SpawnAIFromClass` "/Game/AI/Testing/ShootingAi/BP_ShootingEnemy.BP_ShootingEnemy_C" "/Game/AI/Testing/ShootingAi/BT_ShootingEnemy.BT_ShootingEnemy" _returnvalue_location _returnvalue_rotation))))

(fn `UserConstructionScript`)