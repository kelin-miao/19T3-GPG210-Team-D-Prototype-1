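; AI controller for EnemyPatrol pawns that drives their behavior tree and reports when they sense the player.
; On possession it stores the EnemyPatrol reference and runs EnemyPatrolAI_BT.
; Perception updates for BP_Player set the CanSeePlayer blackboard key to whether the stimulus was sensed.
; Walk and Run events forward to the possessed enemy to switch its movement mode.
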(event `self.AIPerception.OnTargetPerceptionUpdated`
  (params (Actor :type "Actor Object Reference") (Stimulus :type "AIStimulus Structure"))
  (cast `/Game/Jonathon_Torres/Blueprints/BP_Player` Actor)
  (`BlackboardComponent.SetValueAsBool` (`AIBlueprintHelperLibrary.GetBlackboard` null) "CanSeePlayer" (`.bSuccessfullySensed` (break `AIStimulus` Stimulus))))

(event `Walk`
  (`/Game/Jonathon_Torres/Blueprints/EnemyPatrol/EnemyPatrol.Walk` (`self.EnemyPatrol`)))

(event `Run`
  (`/Game/Jonathon_Torres/Blueprints/EnemyPatrol/EnemyPatrol.Run` (`self.EnemyPatrol`)))

(event `self.ReceivePossess`
  (params (PossessedPawn :type "Pawn Object Reference"))
  (bind _asenemy_patrol (cast `/Game/Jonathon_Torres/Blueprints/EnemyPatrol/EnemyPatrol` PossessedPawn))
  (set `self.EnemyPatrol` _asenemy_patrol)
  (`self.RunBehaviorTree` "/Game/Jonathon_Torres/Blueprints/EnemyPatrol/EnemyPatrolAI_BT.EnemyPatrolAI_BT"))

(fn `UserConstructionScript`)