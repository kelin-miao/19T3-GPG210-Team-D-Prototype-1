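; EnemyPatrol is a patrolling enemy character with health, two movement speeds and a score reward on death.
; Walk and Run events switch max walk speed, and BeginPlay passes the enemy's reference to its health bar widget.
; TakeDamagePatrol updates clamped health and its percentage, which Tick polls to destroy the actor at zero and add TargetScore through ThirdPersonGameMode.
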(event `Walk`
  (set `CharacterMovementComponent.MaxWalkSpeed` 250.0 (`self.CharacterMovement`)))

(event `Run`
  (set `CharacterMovementComponent.MaxWalkSpeed` 600.0 (`self.CharacterMovement`)))

(event `self.ReceiveBeginPlay`
  ;[1 1 1] HealthBar
  (bind _asenemy_patrol_health_ui (cast `/Game/Jonathon_Torres/Blueprints/Widgets/EnemyPatrolHealthUI` (`WidgetComponent.GetUserWidgetObject` (`self.EnemyPatrolHealthUI`))))
  (set `/Game/Jonathon_Torres/Blueprints/Widgets/EnemyPatrolHealthUI.EnemyPatrol` self _asenemy_patrol_health_ui))

(event `self.ReceiveTick`
  (params (DeltaSeconds :type "Float (single-precision)"))
  ;[1 0.2083 0.2083] WhenTakingDamage
  (`|ExecutionSequence`
    (:`then_1`
      (if (<= (`self.Health Percentage`) 0.0)
        (`self.K2_DestroyActor`)
        (bind _asthird_person_game_mode (cast `/Game/Jonathon_Torres/Blueprints/ThirdPersonGameMode` (`GameplayStatics.GetGameMode`)))
        (`/Game/Jonathon_Torres/Blueprints/ThirdPersonGameMode.AddTargetPoints` _asthird_person_game_mode (`self.Target Score`))))))

(fn `TakeDamagePatrol`
  (params (Damage :type "Float (double-precision)"))
  (bind _output_get (set `self.Health` (`KismetMathLibrary.FClamp` (- (`self.Health`) Damage) 0.0 200.0)))
  (set `self.Health Percentage` (/ _output_get 100.0)))

(fn `UserConstructionScript`)