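; Navigator pawn for the DonNavigation AI samples, driven by a behavior tree and custom movement input.
; A trigger event waits a wake-up delay, then runs the behavior tree on its AI controller once.
; Custom movement input smoothly rotates the pawn toward the travel direction with clamped pitch and roll.
; It then calls AddMovementInput with speed-scaled input but a zero direction vector.
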(event `self.ReceiveTick`
  (params (DeltaSeconds :type "Float (single-precision)")))

(event `self.AddMovementInputCustom`
  (params (WorldDirection :type "Vector Structure") (ScaleValue :type "Float (single-precision)"))
  (`self.K2_SetActorRotation` (`KismetMathLibrary.RInterpTo` (`self.K2_GetActorRotation`) (`KismetMathLibrary.MakeRotator` (`KismetMathLibrary.FClamp` (.roll (`KismetMathLibrary.MakeRotFromX` WorldDirection)) -30.0 30.0) (`KismetMathLibrary.FClamp` (.pitch (`KismetMathLibrary.MakeRotFromX` WorldDirection)) -30.0 30.0) (.yaw (`KismetMathLibrary.MakeRotFromX` WorldDirection))) (`GameplayStatics.GetWorldDeltaSeconds`) 5.0))
  (`self.AddMovementInput` (0.0 0.0 0.0) (* ScaleValue (`self.Bot Speed Scale`))))

(event `CallTriggerActor_1`
  (`KismetSystemLibrary.Delay` (`self.Wake Up Delay`))
  (if (not (`self.BT Initialized`))
    (bind _asaicontroller (cast `AIController` (`self.GetController`)))
    (`AIController.RunBehaviorTree` _asaicontroller (`self.Behavior To Run`))
    (set `self.BT Initialized` true)))

(event `CallTriggerActorEndOverlap_1`)

(fn `UserConstructionScript`)