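; Guard AI enemy that damages the player at close range and adds score to the game mode when destroyed.
; TakeDamage updates a clamped health percentage, and Tick destroys the guard once it reaches zero.
; Tick also runs a horizontal distance check, then applies fixed damage after a short Delay.
; A timeline resets the HitDelay flag, which this graph never reads, and the health-bar widget link is disconnected.
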(event `self.ReceiveBeginPlay`
  ;[1 1 1] HealthBar
)

(event `self.ReceiveTick`
  (params (DeltaSeconds :type "Float (single-precision)"))
  ;[1 0.2083 0.2083] WhenTakingDamage
  (`|ExecutionSequence`
    (:`then_0`
      (if (<= (`self.Health Percentage`) 0.0)
        (`self.K2_DestroyActor`)))
    (:`then_1`
      ;[1 1 1] The Player dies instantly
      (if (`self.destroyed`)
        _
        (elif (`self.IsInAttackRange`)
          (`KismetSystemLibrary.Delay` 0.5)
          (bind _asplayer (cast `/Game/Jonathon_Torres/Blueprints/Player` (`GameplayStatics.GetPlayerPawn` 0)))
          (`/Game/Jonathon_Torres/Blueprints/Player.PlayerTakeDamage` _asplayer 2.5)
          (set `self.HitDelay` true)
          (`Timeline|Timeline_1` :!via `PlayFromStart`
            (:`Finished`
              (set `self.HitDelay` false))))))))

(event `self.ReceiveDestroyed`
  ;[1 1 1] Destroyed
  (set `self.destroyed` true)
  (bind _asthird_person_game_mode (cast `/Game/Jonathon_Torres/Blueprints/ThirdPersonGameMode` (`GameplayStatics.GetGameMode`)))
  (`/Game/Jonathon_Torres/Blueprints/ThirdPersonGameMode.AddTargetPoints` _asthird_person_game_mode (`self.Target Score`)))

(fn `IsInAttackRange`
  (returns (attackRangeCheck :type Boolean))
  (bind (_returnvalue_x _returnvalue_y) (`KismetMathLibrary.BreakVector` (`self.K2_GetActorLocation` (`GameplayStatics.GetPlayerCharacter` 0))))
  (bind (_returnvalue_x_2 _returnvalue_y_2) (`KismetMathLibrary.BreakVector` (`self.K2_GetActorLocation` self)))
  (return (< (`KismetMathLibrary.Sqrt` (+ (`KismetMathLibrary.Square` (- _returnvalue_x _returnvalue_x_2)) (`KismetMathLibrary.Square` (- _returnvalue_y _returnvalue_y_2)))) (`self.attackRange`))))

(fn `TakeDamage`
  (params (Damage :type "Float (double-precision)"))
  (bind _output_get (set `self.Health` (`KismetMathLibrary.FClamp` (- (`self.Health`) Damage) 0.0 100.0)))
  (set `self.Health Percentage` (/ _output_get 100.0)))

(fn `UserConstructionScript`)