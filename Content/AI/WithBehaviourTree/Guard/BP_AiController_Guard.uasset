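; AI controller for the guard enemy, running the BT_Guard behavior tree.
; On begin play it caches the controlled guard pawn and seeds the blackboard with its patrol path looping flag and a wait timer.
; AI perception updates for the player write visibility and last stimulus location to the blackboard.
; Tick stores the current move status in MovementStatus.
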(event `self.ReceiveBeginPlay`
  (bind _returnvalue (`AIBlueprintHelperLibrary.GetBlackboard` null))
  (`self.RunBehaviorTree` "/Game/AI/WithBehaviourTree/Guard/BT_Guard.BT_Guard")
  (bind _asbp_ai_guard (cast `/Game/AI/WithBehaviourTree/Guard/BP_Ai_Guard` (`self.K2_GetPawn`)))
  (bind _output_get (set `self.aiReference` _asbp_ai_guard))
  (`BlackboardComponent.SetValueAsBool` _returnvalue "PatrolPathLooping" (`/Game/AI/WithBehaviourTree/Guard/BP_PatrolPoint_Guards.isLooping` (`/Game/AI/WithBehaviourTree/Guard/BP_Ai_Guard.patrolPoints` _output_get)))
  (`BlackboardComponent.SetValueAsFloat` _returnvalue "WaitTimer" 3.0))

(event `self.AIPerception.OnTargetPerceptionUpdated`
  (params (Actor :type "Actor Object Reference") (Stimulus :type "AIStimulus Structure"))
  (bind (_age _expirationage _strength _stimuluslocation _receiverlocation _tag _bsuccessfullysensed) (break `AIStimulus` Stimulus))
  (bind _returnvalue (`AIBlueprintHelperLibrary.GetBlackboard` null))
  (bind _asplayer (cast `/Game/ThirdPersonBP/Blueprints/Player` Actor))
  (set `self.playerReference` _asplayer)
  (`BlackboardComponent.SetValueAsBool` _returnvalue "CanSeePlayer" _bsuccessfullysensed)
  (`BlackboardComponent.SetValueAsVector` _returnvalue "WhereLastSeen" _stimuluslocation))

(event `self.ReceiveTick`
  (params (DeltaSeconds :type "Float (single-precision)"))
  (set `self.MovementStatus` (`self.GetMoveStatus`)))

(fn `UserConstructionScript`)