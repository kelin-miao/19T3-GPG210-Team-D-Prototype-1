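; EQS generator that produces cover point candidates around player 0 for shooting AI, ignoring the supplied context locations.
; It traces inward every 5 degrees from a ring at CoverDetectionDistance to find obstacle faces.
; Each hit is offset along its normal and raised, then traced toward the player's upper body.
; Points whose view is blocked by something other than the player become query items, at that raised height.
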(fn `DoItemGeneration`
  (params (ContextLocations :type "Array of Vector Structure (by ref)"))
  (bind _returnvalue (- (`Actor.K2_GetActorLocation` (`GameplayStatics.GetPlayerPawn` 0)) (0.0 0.0 50.0)))
  (`KismetArrayLibrary.Array_Clear` (`self.LocationSet`))
  (for _index (range 72)
    (bind (_outhit _returnvalue_2) (`KismetSystemLibrary.LineTraceSingle` (+ (* (`KismetMathLibrary.GreaterGreater_VectorRotator` (1.0 0.0 0.0) (`KismetMathLibrary.MakeRotator` 0.0 0.0 (* _index 5.0))) (`self.CoverDetectionDistance`)) _returnvalue) _returnvalue "TraceTypeQuery1"))
    (if _returnvalue_2
      (bind (_bblockinghit _binitialoverlap _time _distance _location _impactpoint _normal _impactnormal) (`GameplayStatics.BreakHitResult` _outhit))
      (bind (_outhit_2 _returnvalue_3) (`KismetSystemLibrary.LineTraceSingle` (+ _impactpoint (* _impactnormal 50.0) (0.0 0.0 125.0)) (+ (`Actor.K2_GetActorLocation` (`GameplayStatics.GetPlayerPawn` 0)) (0.0 0.0 75.0)) "TraceTypeQuery1"))
      (bind (_bblockinghit_2 _binitialoverlap_2 _time_2 _distance_2 _location_2 _impactpoint_2 _normal_2 _impactnormal_2 _physmat _hitactor _hitcomponent _hitbonename _hititem _faceindex _tracestart) (`GameplayStatics.BreakHitResult` _outhit_2))
      (if (and _returnvalue_3 (!= _hitactor (`GameplayStatics.GetPlayerPawn` 0)))
        (`KismetArrayLibrary.Array_Add` (`self.LocationSet`) _tracestart))))
  (for _array_element (`self.LocationSet`)
    (`self.AddGeneratedVector` _array_element))
  (return))