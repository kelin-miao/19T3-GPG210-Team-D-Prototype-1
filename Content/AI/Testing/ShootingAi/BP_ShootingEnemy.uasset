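; Shooting AI enemy that fires at the player, takes bullet damage and dodges when threatened.
; Shoot traces toward a random point around the player, then spawns a laser bullet along that line with sound.
; Player bullet damage lowers health until it explodes and is destroyed.
; Player ThreatDetection point damage triggers, after a short delay, traces across its rear half-circle and AI moves toward randomly picked unblocked points, gated by a DoOnce.
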(event `StopMovement`
  ;[1 1 1] Stop Movement
  (`MovementComponent.StopMovementImmediately` (`self.CharacterMovement`)))

(event `Shoot`
  (bind (_returnvalue_x _returnvalue_y _returnvalue_z) (`KismetMathLibrary.BreakVector` (`self.K2_GetActorLocation` (`GameplayStatics.GetPlayerPawn` 0))))
  ;[1 1 1] Shoot
  (`/Engine/EditorBlueprintResources/StandardMacros.DoOnce` false :!label _label
    (:`Completed`
      (bind _outhit (`KismetSystemLibrary.LineTraceSingle` (`SceneComponent.K2_GetComponentLocation` (`self.ForwardArrow`)) (`KismetMathLibrary.RandomPointInBoundingBox` (`KismetMathLibrary.MakeVector` _returnvalue_x _returnvalue_y (+ _returnvalue_z 30.0)) (40.0 40.0 20.0)) "TraceTypeQuery1"))
      (bind (_bblockinghit _binitialoverlap _time _distance _location _impactpoint _normal _impactnormal _physmat _hitactor _hitcomponent _hitbonename _hititem _faceindex _tracestart _traceend) (`GameplayStatics.BreakHitResult` _outhit))
      (`GameplayStatics.PlaySoundAtLocation` "/Game/AI/Testing/ShootingAi/sound_effects/pew_pew_laser.pew_pew_laser" _tracestart (struct) 0.2 1.0 0.0 null null null)
      (`|SpawnActorFromClass` "/Game/AI/Testing/ShootingAi/BP_LaserBullet.BP_LaserBullet_C" (`KismetMathLibrary.MakeTransform` _tracestart (`KismetMathLibrary.FindLookAtRotation` _tracestart _traceend) (4.0 4.0 1.0)) "Undefined" "OverrideRootScale" null null)
      (`self.ResetShoot`))))

(event `ResetShoot`
  ;[1 1 1] Shoot
  (goto _label :!via `Reset`))

(event `self.ReceiveAnyDamage`
  (params (Damage :type "Float (single-precision)") (DamageType :type "DamageType Object Reference") (InstigatedBy :type "Controller Object Reference") (DamageCauser :type "Actor Object Reference"))
  ;[1 1 1] Get Hit
  (if (and (== (`GameplayStatics.GetObjectClass` DamageType) "/Game/AI/Testing/ShootingAi/DmgTypeBP_BulletDamage.DmgTypeBP_BulletDamage_C") (== DamageCauser (`GameplayStatics.GetPlayerPawn` 0)))
    (set `self.Health Percentage` (- (`self.Health Percentage`) Damage))
    (`GameplayStatics.PlaySoundAtLocation` "/Game/Jonathon_Torres/Blueprints/small_explosion.small_explosion" (`self.K2_GetActorLocation`) (struct) 1.0 1.0 0.0 null null null)
    (if (<= (`self.Health Percentage`) 0.0)
      (`GameplayStatics.SpawnEmitterAtLocation` "/Game/StarterContent/Particles/P_Explosion.P_Explosion" (`self.K2_GetActorLocation`) (struct) (2.0 2.0 2.0))
      (`self.K2_DestroyActor`))))

(event `self.ReceivePointDamage`
  (params (Damage :type "Float (single-precision)") (DamageType :type "DamageType Object Reference") (HitLocation :type "Vector Structure") (HitNormal :type "Vector Structure") (HitComponent :type "PrimitiveComponent Object Reference") (BoneName :type Name) (ShotFromDirection :type "Vector Structure") (InstigatedBy :type "Controller Object Reference") (DamageCauser :type "Actor Object Reference") (HitInfo :type "HitResult Structure (by ref)"))
  (bind _returnvalue (`self.K2_GetActorLocation`))
  (bind (_returnvalue_roll _returnvalue_pitch _returnvalue_yaw) (`KismetMathLibrary.BreakRotator` (`self.K2_GetActorRotation`)))
  (bind _strafevectors (`self.StrafeVectors`))
  ;[1 1 1] Strafe when threatened
  (if (and (== (`GameplayStatics.GetObjectClass` DamageType) "/Game/AI/Testing/ShootingAi/DmgTypeBP_ThreatDetection.DmgTypeBP_ThreatDetection_C") (== DamageCauser (`GameplayStatics.GetPlayerPawn` 0)))
    (`KismetSystemLibrary.Delay` 0.2)
    (`/Engine/EditorBlueprintResources/StandardMacros.DoOnce` false :!label _label_2
      (:`Completed`
        (`KismetArrayLibrary.Array_Clear` (`self.StrafeVectors`))
        (for _index (range 11)
          (bind (_outhit _returnvalue_2) (`KismetSystemLibrary.LineTraceSingle` _returnvalue (+ _returnvalue (* (`KismetMathLibrary.GreaterGreater_VectorRotator` (0.0 1.0 0.0) (`KismetMathLibrary.MakeRotator` 0.0 0.0 (+ _returnvalue_yaw (* _index 18.0)))) 200.0)) "TraceTypeQuery1"))
          (if (not _returnvalue_2)
            (bind _returnvalue_3 (`KismetArrayLibrary.Array_Add` _strafevectors (`.TraceEnd` (`GameplayStatics.BreakHitResult` _outhit))))
            (`|AIMoveTo` self (`|GetArrayItem` _strafevectors (`KismetMathLibrary.RandomInteger` _returnvalue_3)) null 1.0
              (:`OnSuccess`
                _)
              (:`OnFail`
                _))
            (`self.ResetStrafe`)))))))

(event `ResetStrafe`
  ;[1 1 1] Strafe when threatened
  (goto _label_2 :!via `Reset`))

(fn `UserConstructionScript`)