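; BP_LaserBullet is a laser projectile in the ShootingAi test folder that damages the player on contact.
; When BulletMesh overlaps the first player character, it spawns a half-scale explosion at the player's location, applies Damage and destroys itself.
; It ignores every other actor, with an explicit cast check that skips BP_ShootingEnemy.
; On BeginPlay it starts a Lifetime delay, after which it destroys itself.
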(event `self.BulletMesh.OnComponentBeginOverlap`
  (params (OverlappedComponent :type "PrimitiveComponent Object Reference") (OtherActor :type "Actor Object Reference") (OtherComp :type "PrimitiveComponent Object Reference") (OtherBodyIndex :type Integer) (bFromSweep :type Boolean) (SweepResult :type "HitResult Structure (by ref)"))
  (cast `/Game/AI/Testing/ShootingAi/BP_ShootingEnemy` OtherActor
    (:`CastFailed`
      (if (== OtherActor (`GameplayStatics.GetPlayerCharacter` 0))
        (`GameplayStatics.SpawnEmitterAtLocation` "/Game/StarterContent/Particles/P_Explosion.P_Explosion" (`self.K2_GetActorLocation` OtherActor) (struct) (0.5 0.5 0.5))
        (`GameplayStatics.ApplyDamage` (`GameplayStatics.GetPlayerCharacter` 0) (`self.Damage`) null self "/Script/Engine.DamageType")
        (`self.K2_DestroyActor`)))))

(event `self.ReceiveBeginPlay`
  (`KismetSystemLibrary.Delay` (`self.Lifetime`))
  (`self.K2_DestroyActor`))

(fn `UserConstructionScript`)