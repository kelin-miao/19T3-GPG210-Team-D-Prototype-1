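; Guard enemy AI character that fires a laser beam at the player and awards score when destroyed.
; Tick checks player distance, then uses delays to apply damage and toggle the beam from its forward arrow; HitDelay is set but never read.
; Only the player's bullet damage lowers HealthPercentage, destroying the guard at zero and adding TargetScore to ThirdPersonGameMode.
; BeginPlay links the health widget; TakeDamage and IsInAttackRange go uncalled here.
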(event `self.ReceiveBeginPlay`
  ;[0.1681 1 0.1843] HealthBar
  (`|ExecutionSequence`
    (:`then_0`
      (set `self.Tags` (`|MakeArray` "Enemy" :!type "Name"))
      (`ActorComponent.Deactivate` (`self.LaserBeam`)))
    (:`then_1`
      (bind _asai_guard_health_ui (cast `/Game/Jonathon_Torres/Blueprints/Widgets/AI_GuardHealthUI` (`WidgetComponent.GetUserWidgetObject` (`self.Widget`))))
      (set `/Game/Jonathon_Torres/Blueprints/Widgets/AI_GuardHealthUI.BP_AI_Guard` self _asai_guard_health_ui))))

(event `DestroyObject`
  ;[0.1122 0.2849 1] After the enemy gets destory, it stores points into the gamemode and update my score system
  (set `self.destroyed` true :!label _label)
  (bind _asthird_person_game_mode (cast `/Game/Jonathon_Torres/Blueprints/ThirdPersonGameMode` (`GameplayStatics.GetGameMode`)))
  (`/Game/Jonathon_Torres/Blueprints/ThirdPersonGameMode.AddTargetPoints` _asthird_person_game_mode (`self.Target Score`)))

(event `self.ReceiveDestroyed`
  ;[0.1122 0.2849 1] After the enemy gets destory, it stores points into the gamemode and update my score system
  (goto _label))

(event `self.ReceiveTick`
  (params (DeltaSeconds :type "Float (single-precision)"))
  (bind _laserbeam (`self.LaserBeam`))
  ;[1 0.131 0.3697] When player takes damage
  (if (`self.destroyed`)
    _
    (elif (< (`self.GetDistanceTo` (`GameplayStatics.GetPlayerPawn` 0)) (`self.attackRange`))
      (`KismetSystemLibrary.Delay` 0.5)
      (`ActorComponent.Activate` _laserbeam false)
      (`ParticleSystemComponent.SetBeamSourcePoint` _laserbeam 0 (`SceneComponent.K2_GetComponentLocation` (`self.ForwardArrow`)) 0)
      (`ParticleSystemComponent.SetBeamTargetPoint` _laserbeam 0 (`self.K2_GetActorLocation` (`GameplayStatics.GetPlayerPawn` 0)) 0)
      (`GameplayStatics.ApplyDamage` (`GameplayStatics.GetPlayerPawn` 0) (`self.Attack Damage`))
      (`KismetSystemLibrary.Delay` 1.5)
      (`ActorComponent.Deactivate` _laserbeam)
      (set `self.HitDelay` true)
      (`Timeline|Timeline_1` :!via `PlayFromStart`
        (:`Finished`
          (set `self.HitDelay` false))))))

(event `self.ReceiveAnyDamage`
  (params (Damage :type "Float (single-precision)") (DamageType :type "DamageType Object Reference") (InstigatedBy :type "Controller Object Reference") (DamageCauser :type "Actor Object Reference"))
  (if (and (== (`GameplayStatics.GetObjectClass` DamageType) "/Game/AI/Testing/ShootingAi/DmgTypeBP_BulletDamage.DmgTypeBP_BulletDamage_C") (== DamageCauser (`GameplayStatics.GetPlayerPawn` 0)))
    (set `self.Health Percentage` (- (`self.Health Percentage`) Damage))
    (if (<= (`self.Health Percentage`) 0.0)
      (`self.K2_DestroyActor`))))

(fn `getch`
  (returns (NewParam :type "CharacterMovementComponent Object Reference"))
  (return (`self.CharacterMovement`)))

(fn `IsInAttackRange`
  (returns (attackRangeCheck :type Boolean))
  (bind (_returnvalue_x _returnvalue_y) (`KismetMathLibrary.BreakVector` (`self.K2_GetActorLocation` (`GameplayStatics.GetPlayerCharacter` 0))))
  (bind (_returnvalue_x_2 _returnvalue_y_2) (`KismetMathLibrary.BreakVector` (`self.K2_GetActorLocation` self)))
  (return (< (`KismetMathLibrary.Sqrt` (+ (`KismetMathLibrary.Square` (- _returnvalue_x _returnvalue_x_2)) (`KismetMathLibrary.Square` (- _returnvalue_y _returnvalue_y_2)))) (`self.attackRange`))))

(fn `TakeDamage`
  (params (Damage :type "Float (double-precision)"))
  (bind _output_get (set `self.Health` (`KismetMathLibrary.FClamp` (- (`self.Health`) Damage) 0.0 100.0)))
  (set `self.Health Percentage` (/ _output_get 100.0)))

(fn `UserConstructionScript`)