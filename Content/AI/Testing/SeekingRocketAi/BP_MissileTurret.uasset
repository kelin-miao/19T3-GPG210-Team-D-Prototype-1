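; BP_MissileTurret is a test turret that spawns a seeking rocket when a TwinStickPawnV2 enters its capsule.
; The overlap ignores the pawn's HitBox component, spawns BP_SeekingRocket at the Arrow's location with a fixed rotation, and prints a debug message.
; Tick pulses the MissileSilo's dynamic material between two colours using the absolute value of a looping counter, and applies the emissive brightness.
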(event `self.ReceiveBeginPlay`
  (bind _returnvalue (`KismetMaterialLibrary.CreateDynamicMaterialInstance` "/Game/AI/Testing/SeekingRocketAi/materials/MTI_EColourChange.MTI_EColourChange"))
  (bind _output_get (set `self.MaterialInstance` _returnvalue))
  (`PrimitiveComponent.SetMaterial` (`self.Missile_Silo`) 0 _output_get))

(event `self.Capsule.OnComponentBeginOverlap`
  (params (OverlappedComponent :type "PrimitiveComponent Object Reference") (OtherActor :type "Actor Object Reference") (OtherComp :type "PrimitiveComponent Object Reference") (OtherBodyIndex :type Integer) (bFromSweep :type Boolean) (SweepResult :type "HitResult Structure (by ref)"))
  (bind _returnvalue_location (`KismetMathLibrary.BreakTransform` (`SceneComponent.K2_GetComponentToWorld` (`self.Arrow`))))
  (bind _astwin_stick_pawn_v2 (cast `/Game/TwinStickBP/Blueprints/TwinStickPawnV2` OtherActor))
  (if (not (== (`/Game/TwinStickBP/Blueprints/TwinStickPawnV2.HitBox` _astwin_stick_pawn_v2) OtherComp))
    (`|SpawnActorFromClass` "/Game/AI/Testing/SeekingRocketAi/BP_SeekingRocket.BP_SeekingRocket_C" (`KismetMathLibrary.MakeTransform` _returnvalue_location (struct :`Pitch` 90.0)) "AlwaysSpawn" "OverrideRootScale" null null)
    (`KismetSystemLibrary.PrintString` "spawned")))

(event `self.ReceiveTick`
  (params (DeltaSeconds :type "Float (single-precision)"))
  (bind _materialinstance (`self.MaterialInstance`))
  (bind _alphavalue (`self.AlphaValue`))
  ;[1 1 1] Colour Changing
  (if (and (<= -100.0 _alphavalue) (<= _alphavalue 100.0))
    (set `self.AlphaValue` (- (`self.AlphaValue`) 2.0))
    (else
      (set `self.AlphaValue` 100.0)))
  (`MaterialInstanceDynamic.SetVectorParameterValue` _materialinstance "Colour" (`KismetMathLibrary.LinearColorLerp` (`KismetMathLibrary.Conv_ColorToLinearColor` (`self.ColourOne`)) (`KismetMathLibrary.Conv_ColorToLinearColor` (`self.ColourTwo`)) (/ (`KismetMathLibrary.Abs` (`self.AlphaValue`)) 100.0)))
  (`MaterialInstanceDynamic.SetScalarParameterValue` _materialinstance "EmissionValue" (`self.EmissiveBrightness`)))

(fn `UserConstructionScript`)