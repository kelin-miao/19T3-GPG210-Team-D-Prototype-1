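; BP_Light is a light actor in the distance test map whose emissive material changes colour with the player's proximity and pulses in intensity.
; BeginPlay applies a dynamic instance of MT_Light_Emissive and picks a random time offset.
; Each Tick blends base and emissive colour from CloseColour to FarColour by buffered, clamped player distance, while an offset sine wave drives intensity.
; An unconnected sine-based colour-cycling chain never runs.
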(event `self.ReceiveBeginPlay`
  (bind _returnvalue (`KismetMaterialLibrary.CreateDynamicMaterialInstance` "/Game/Levels/Maps/Light_Distance_Test/Materials/MT_Light_Emissive.MT_Light_Emissive"))
  (bind _output_get (set `self.Dynamic Material` _returnvalue))
  (`PrimitiveComponent.SetMaterial` (`self.Light`) 0 _output_get)
  (bind _output_get_2 (set `self.Random Offset` (`KismetMathLibrary.RandomFloatInRange` 0.0 5.0))))

(event `self.ReceiveTick`
  (params (DeltaSeconds :type "Float (single-precision)"))
  (bind _dynamic_material (`self.Dynamic Material`))
  (bind _returnvalue_location (`KismetMathLibrary.BreakTransform` (`self.GetTransform` (`GameplayStatics.GetPlayerCharacter` 0))))
  (bind _returnvalue_location_2 (`KismetMathLibrary.BreakTransform` (`SceneComponent.K2_GetComponentToWorld` (`self.Light`))))
  (bind _returnvalue (`KismetMathLibrary.LinearColorLerp` (`KismetMathLibrary.Conv_ColorToLinearColor` (`self.Close Colour`)) (`KismetMathLibrary.Conv_ColorToLinearColor` (`self.Far Colour`)) (`KismetMathLibrary.FClamp` (/ (- (`KismetMathLibrary.Vector_Distance` _returnvalue_location_2 _returnvalue_location) (`self.Distance Buffer`)) (`self.Distance To Light`)))))
  (`MaterialInstanceDynamic.SetVectorParameterValue` _dynamic_material "Emissive Colour" _returnvalue)
  (`MaterialInstanceDynamic.SetVectorParameterValue` _dynamic_material "Base Colour" _returnvalue)
  (`MaterialInstanceDynamic.SetScalarParameterValue` _dynamic_material "Intensity" (`KismetMathLibrary.Lerp` (`self.Max Intensity`) (`self.Min Intensity`) (/ (+ (`KismetMathLibrary.Sin` (/ (+ (`GameplayStatics.GetTimeSeconds`) (stale `self.ReceiveBeginPlay` _output_get_2)) (`self.Intensity Time Cycle`))) 1.0) 2.0))))

(fn `UserConstructionScript`)