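; Procedural city-block spawner for a generator test map that builds a stacked grid of instanced motif meshes in its construction script.
; Each grid cell gets a half-tile offset tower at randomized height, then one of four motifs per level with random right-angle yaw.
; Support meshes alternate with their reversed variant in a checkerboard.
; Motif selection re-rolls the random number at each branch, so the four variants are unevenly weighted.
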(event `self.ReceiveTick`
  (params (DeltaSeconds :type "Float (single-precision)")))

(event `self.ReceiveBeginPlay`)

(fn `UserConstructionScript`
  (bind _returnvalue (`KismetMathLibrary.RandomInteger` 3))
  (bind _tile_multiplier (`self.Tile Multiplier`))
  (bind _motif_distance (`self.Motif Distance`))
  (bind _returnvalue_2 (- _tile_multiplier 1))
  (bind _returnvalue_3 (/ _motif_distance 2.0))
  (bind _returnvalue_4 (* _tile_multiplier _returnvalue_3))
  (bind _returnvalue_5 (`KismetMathLibrary.MakeRotator` 0.0 0.0 (* (`KismetMathLibrary.RandomInteger` 3) 90.0)))
  (for _index (range (+ _returnvalue_2 1))
    (for _index_2 (range (+ _returnvalue_2 1))
      (`|ExecutionSequence`
        (:`then_0`
          (bind _returnvalue_6 (- _returnvalue_4 (* _index _motif_distance)))
          (bind _returnvalue_7 (- _returnvalue_4 (* _index_2 _motif_distance)))
          (`InstancedStaticMeshComponent.AddInstance` (`self.Tower Instance`) (`KismetMathLibrary.MakeTransform` (`KismetMathLibrary.MakeVector` (+ _returnvalue_3 _returnvalue_6) (+ _returnvalue_3 _returnvalue_7) (+ (+ (`KismetMathLibrary.RandomFloatInRange` 0.0 300.0) -1100.0) (`self.Motif Level Height`))))))
        (:`then_1`
          (for _index_3 (range (`self.Motif Levels`))
            (if (== _returnvalue 0)
              (bind _returnvalue_8 (`KismetMathLibrary.MakeVector` _returnvalue_6 _returnvalue_7 (* _index_3 (`self.Level Height`))))
              (`InstancedStaticMeshComponent.AddInstance` (`self.Motif 1 Instance`) (`KismetMathLibrary.MakeTransform` _returnvalue_8 _returnvalue_5))
              (elif (== _returnvalue 1)
                (`InstancedStaticMeshComponent.AddInstance` (`self.Motif 2 Instance`) (`KismetMathLibrary.MakeTransform` _returnvalue_8 _returnvalue_5))
                (elif (== _returnvalue 2)
                  (`InstancedStaticMeshComponent.AddInstance` (`self.Motif 3 Instance`) (`KismetMathLibrary.MakeTransform` _returnvalue_8 _returnvalue_5))
                  (else
                    (`InstancedStaticMeshComponent.AddInstance` (`self.Motif 4 Instance`) (`KismetMathLibrary.MakeTransform` _returnvalue_8 _returnvalue_5))))))
            (if (`KismetMathLibrary.Conv_IntToBool` (mod (+ _index _index_2) 2))
              (`InstancedStaticMeshComponent.AddInstance` (`self.Support Instance`) (`KismetMathLibrary.MakeTransform` _returnvalue_8 (`KismetMathLibrary.MakeRotator` 0.0)))
              (else
                (`InstancedStaticMeshComponent.AddInstance` (`self.SupportReverse Instance`) (`KismetMathLibrary.MakeTransform` _returnvalue_8 (`KismetMathLibrary.MakeRotator` 0.0)))))))))))