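; Test spawner that streams an endless procedural city of motifs, random-height towers and ground tiles on a grid around the TwinStickPawnV2 player.
; BeginPlay creates one HISM component per configured mesh and fills the view square with randomly chosen instances, stacking tower levels by mesh bounds beneath a roof.
; Tick detects grid-cell changes, then removes out-of-range instances and spawns missing cells, using a spawned-points list to track occupied cells.
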(event `self.ReceiveBeginPlay`
  (bind _outactors (`GameplayStatics.GetAllActorsOfClass` "/Game/TwinStickBP/Blueprints/TwinStickPawnV2.TwinStickPawnV2_C"))
  (set `self.Player Ref` (`|GetArrayItem` _outactors))
  (`self.Init All HISM component Static Mesh`)
  (`self.Initialise View Area` 0.0))

(event `Check HISM Valid Event`
  (params (Array :type "Array of HierarchicalInstancedStaticMeshComponent Object Reference"))
  (for _array_element Array
    (for _index (range (`InstancedStaticMeshComponent.GetInstanceCount` _array_element))
      (bind _remove_ (`self.Remove?` (.location (`InstancedStaticMeshComponent.GetInstanceTransform` _array_element _index true))))
      (if _remove_
        (`InstancedStaticMeshComponent.RemoveInstance` _array_element _index)))))

(event `self.ReceiveTick`
  (params (DeltaSeconds :type "Float (single-precision)"))
  (`self.Update Player Point Position`))

(fn ` Init HISM component Static Mesh`
  (params (`Static Mesh Array` :type "Array of StaticMesh Object Reference") (`HISM Component Array` :type "Array of HierarchicalInstancedStaticMeshComponent Object Reference"))
  (for _array_element `Static Mesh Array`
    (bind _returnvalue (`AddComponent|NODE_AddHierarchicalInstancedStaticMeshComponent-0`))
    (`KismetArrayLibrary.Array_Add` `HISM Component Array` _returnvalue)
    (`StaticMeshComponent.SetStaticMesh` _returnvalue _array_element)))

(fn `Check All HISM Valid`
  (`self.Check HISM Valid` (`self.HISM Motif Components`))
  (`self.Check HISM Valid` (`self.HISM Tower Level Components`))
  (`self.Check HISM Valid` (`self.HISM Tower Roof Components`))
  (`self.Check HISM Valid` (`self.HISM Ground Level Components`))
  (return))

(fn `Check HISM Valid`
  (params (`HSIM Array` :type "Array of HierarchicalInstancedStaticMeshComponent Object Reference"))
  (for _array_element `HSIM Array`
    (for _index (range (`InstancedStaticMeshComponent.GetInstanceCount` _array_element))
      (bind _remove_ (`self.Remove?` (.location (`InstancedStaticMeshComponent.GetInstanceTransform` _array_element _index true))))
      (if _remove_
        (`InstancedStaticMeshComponent.RemoveInstance` _array_element _index)))))

(fn `Init All HISM component Static Mesh`
  (`self. Init HISM component Static Mesh` (`self.Static Mesh Motifs`) (`self.HISM Motif Components`))
  (`self. Init HISM component Static Mesh` (`self.Static Mesh Tower Level`) (`self.HISM Tower Level Components`))
  (`self. Init HISM component Static Mesh` (`self.Static Mesh Tower Roof`) (`self.HISM Tower Roof Components`))
  (`self. Init HISM component Static Mesh` (`self.Static Mesh Ground Level`) (`self.HISM Ground Level Components`)))

(fn `Initialise View Area`
  (params (Height :type "Float (double-precision)") (`Player Point` :type "IntPoint Structure"))
  (bind _tile_view_distance (`self.Tile View Distance`))
  (bind _returnvalue (* _tile_view_distance -1))
  (for _index (range (+ `Player Point_X` _returnvalue) (+ (+ `Player Point_X` _tile_view_distance) 1))
    (for _index_2 (range (+ _returnvalue `Player Point_Y`) (+ (+ _tile_view_distance `Player Point_Y`) 1))
      (`self.Spawn Point` _index _index_2 Height))))

(fn `Remove?`
  (params (`Object Position` :type "Vector Structure"))
  (returns (`Remove?` :type Boolean))
  (bind (_returnvalue_x _returnvalue_y) (`KismetMathLibrary.BreakVector` (`self.K2_GetActorLocation` (`self.Player Ref`))))
  (bind _returnvalue (* (+ (`self.Tile View Distance`) 1) (`self.Motif Distance`)))
  (return (or (> (`KismetMathLibrary.Abs` (- _returnvalue_x `Object Position_X`)) _returnvalue) (> (`KismetMathLibrary.Abs` (- _returnvalue_y `Object Position_Y`)) _returnvalue))))

(fn `Spawn Point`
  (params (`Location Int X` :type Integer) (`Location Int Y` :type Integer) (`Location Z` :type "Float (double-precision)"))
  (bind _motif_distance (`self.Motif Distance`))
  (bind _hism_ground_level_components (`self.HISM Ground Level Components`))
  (bind _hism_tower_level_components (`self.HISM Tower Level Components`))
  (bind _hism_motif_components (`self.HISM Motif Components`))
  (bind _returnvalue (* `Location Int Y` _motif_distance))
  (bind _returnvalue_2 (* `Location Int X` _motif_distance))
  (bind _returnvalue_3 (`KismetMathLibrary.RandomIntegerInRange` 0 (- (`KismetArrayLibrary.Array_Length` _hism_tower_level_components) 1)))
  (for _index (range (`self.Motif Levels`))
    (`InstancedStaticMeshComponent.AddInstance` (`|GetArrayItem` _hism_motif_components (`KismetMathLibrary.RandomIntegerInRange` 0 (- (`KismetArrayLibrary.Array_Length` _hism_motif_components) 1))) (`KismetMathLibrary.MakeTransform` (`KismetMathLibrary.MakeVector` _returnvalue_2 _returnvalue (+ `Location Z` (* _index (`self.Level Height`)))) (`KismetMathLibrary.MakeRotator` 0.0))) ; Motif
  )
  (`self.Spawn Tower` (`|GetArrayItem` _hism_tower_level_components _returnvalue_3) (`|GetArrayItem` (`self.HISM Tower Roof Components`) _returnvalue_3) _returnvalue_2 _returnvalue (* (`KismetMathLibrary.RandomIntegerInRange` 0 7) 45.0) (`KismetMathLibrary.RandomFloatInRange` (`self.Tower Min Height`) (`self.Tower Max Height`)))
  (bind _returnvalue_4 (`InstancedStaticMeshComponent.AddInstance` (`|GetArrayItem` _hism_ground_level_components (`KismetMathLibrary.RandomIntegerInRange` 0 (- (`KismetArrayLibrary.Array_Length` _hism_ground_level_components) 1))) (`KismetMathLibrary.MakeTransform` (`KismetMathLibrary.MakeVector` _returnvalue_2 _returnvalue) (`KismetMathLibrary.MakeRotator` 0.0 0.0 (* (`KismetMathLibrary.RandomInteger` 3) 90.0))))) ; Ground Level
  (`KismetArrayLibrary.Array_Add` (`self.Spawned Points Array`) (make `IntPoint` `Location Int X` `Location Int Y`)))

(fn `Spawn Tower`
  (params (`HISM Level` :type "InstancedStaticMeshComponent Object Reference") (`HISM Roof` :type "InstancedStaticMeshComponent Object Reference") (InstanceTransform_Location_X :type "Float (double-precision)") (InstanceTransform_Location_Y :type "Float (double-precision)") (InstanceTransform_Rotation_Yaw :type "Float (double-precision)") (`Tower Height` :type "Float (double-precision)"))
  (bind (_min _max) (`StaticMeshComponent.GetLocalBounds` `HISM Level`))
  (bind _returnvalue (- (.z _max) (.z _min)))
  (bind _returnvalue_2 (`KismetMathLibrary.Round` (/ `Tower Height` _returnvalue)))
  (for _index (range _returnvalue_2)
    (`InstancedStaticMeshComponent.AddInstance` `HISM Level` (`KismetMathLibrary.MakeTransform` (`KismetMathLibrary.MakeVector` InstanceTransform_Location_X InstanceTransform_Location_Y (* _index _returnvalue)) (`KismetMathLibrary.MakeRotator` 0.0 0.0 InstanceTransform_Rotation_Yaw))) ; Level
  )
  (`InstancedStaticMeshComponent.AddInstance` `HISM Roof` (`KismetMathLibrary.MakeTransform` (`KismetMathLibrary.MakeVector` InstanceTransform_Location_X InstanceTransform_Location_Y (* _returnvalue_2 _returnvalue)) (`KismetMathLibrary.MakeRotator` 0.0 0.0 InstanceTransform_Rotation_Yaw))) ; Roof
)

(fn `Update Player Point Position`
  (bind _motif_distance (`self.Motif Distance`))
  (bind (_player_point_position_x _player_point_position_y) (break `IntPoint` (`self.Player Point Position`)))
  (bind (_returnvalue_x _returnvalue_y) (`KismetMathLibrary.BreakVector` (`self.K2_GetActorLocation` (`self.Player Ref`))))
  (bind _returnvalue (`KismetMathLibrary.Round` (/ _returnvalue_y _motif_distance)))
  (bind _returnvalue_2 (`KismetMathLibrary.Round` (/ _returnvalue_x _motif_distance)))
  (if (or (!= _returnvalue_2 _player_point_position_x) (!= _returnvalue _player_point_position_y))
    (set `self.Player Point Position` (make `IntPoint` _returnvalue_2 _returnvalue))
    (`self.Check All HISM Valid`)
    (`self.Update View Area`)
    (`self.Update Spawned Points Array`))
  (return))

(fn `Update Spawned Points Array`
  (bind (_player_point_position_x _player_point_position_y) (break `IntPoint` (`self.Player Point Position`)))
  (bind _tile_view_distance (`self.Tile View Distance`))
  (bind _spawned_points_array (`self.Spawned Points Array`))
  (for (_ _array_index) _spawned_points_array
    (bind (_output_x _output_y) (break `IntPoint` (`|GetArrayItem` _spawned_points_array _array_index)))
    (if (or (> (`KismetMathLibrary.Abs_Int` (- _player_point_position_x _output_x)) _tile_view_distance) (> (`KismetMathLibrary.Abs_Int` (- _player_point_position_y _output_y)) _tile_view_distance))
      (`KismetArrayLibrary.Array_Remove` _spawned_points_array _array_index))))

(fn `Update View Area`
  (bind (_player_point_position_x _player_point_position_y) (break `IntPoint` (`self.Player Point Position`)))
  (bind _tile_view_distance (`self.Tile View Distance`))
  (bind _returnvalue (* _tile_view_distance -1))
  (for _index (range (+ _player_point_position_x _returnvalue) (+ (+ _player_point_position_x _tile_view_distance) 1))
    (for _index_2 (range (+ _player_point_position_y _returnvalue) (+ (+ _player_point_position_y _tile_view_distance) 1))
      (if (not (`KismetArrayLibrary.Array_Contains` (`self.Spawned Points Array`) (make `IntPoint` _index _index_2)))
        (`self.Spawn Point` _index _index_2)))))

(fn `UserConstructionScript`)