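; Spawns flying-car traffic in stacked, two-way lanes along X and Y on a grid that follows the TwinStickPawnV2 player.
; A looping timer adds HISM instances with random offsets at the edges around the player's grid cell, staggering X and Y layers in height.
; Tick moves whole HISM components rather than individual cars.
; When the player changes cell, instances beyond the visible distance are removed.
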(event `self.ReceiveBeginPlay`
  (bind (_returnvalue_x _returnvalue_y _returnvalue_z) (`KismetMathLibrary.BreakVector` (`self.K2_GetActorLocation`)))
  ;[1 1 1] Get Player Ref
  (bind _outactors (`GameplayStatics.GetAllActorsOfClass` "/Game/TwinStickBP/Blueprints/TwinStickPawnV2.TwinStickPawnV2_C"))
  (set `self.Player Ref` (`|GetArrayItem` _outactors))
  (`KismetSystemLibrary.K2_SetTimerDelegate` (delegate `Spawn Cars`) 2.0 true)
  (set `self.Start Height` _returnvalue_z))

(event `Spawn Cars`
  (`self.Spawn Car Layers`))

(event `self.ReceiveTick`
  (params (DeltaSeconds :type "Float (single-precision)"))
  (bind _motif_distance (`self.Motif Distance`))
  (bind (_player_motif_point_location_x _player_motif_point_location_y) (break `IntPoint` (`self.Player Motif Point Location`)))
  (bind _visible_distance (`self.Visible Distance`))
  (bind (_returnvalue_x _returnvalue_y) (`KismetMathLibrary.BreakVector` (`self.K2_GetActorLocation` (`self.Player Ref`))))
  (bind (_returnvalue_x_2 _returnvalue_y_2) (`KismetMathLibrary.BreakVector` (`self.K2_GetActorLocation` (`self.Player Ref`))))
  (bind _returnvalue (`KismetMathLibrary.Round` (/ _returnvalue_x_2 _motif_distance)))
  (bind _returnvalue_2 (`KismetMathLibrary.Round` (/ _returnvalue_y_2 _motif_distance)))
  ;[1 1 1] Move HSMI Components
  (`self.Move HISM Components` (* DeltaSeconds (`self.Car Movement Speed`)))
  ;[1 1 1] Update Player Motif Point Location
  (if (or (!= _player_motif_point_location_x _returnvalue) (!= _player_motif_point_location_y _returnvalue_2))
    (set `self.Player Motif Point Location` (make `IntPoint` _returnvalue _returnvalue_2))
    ;[1 1 1] Distance Check
    (for _array_element (`|MakeArray` (`self.Y- Axis Cars`) (`self.Y+ Axis Cars`) (`self.X- Axis Cars`) (`self.X+ Axis Cars`))
      (for _index (range (`InstancedStaticMeshComponent.GetInstanceCount` _array_element))
        (bind _outinstancetransform (`InstancedStaticMeshComponent.GetInstanceTransform` _array_element _index true))
        (if (or (> (`KismetMathLibrary.Abs` (- _returnvalue_x (.x (.location _outinstancetransform)))) _visible_distance) (> (`KismetMathLibrary.Abs` (- _returnvalue_y (.y (.location _outinstancetransform)))) _visible_distance))
          (`InstancedStaticMeshComponent.RemoveInstance` _array_element _index))))))

(fn `Move HISM Component In Axis`
  (params (HISMC :type "HierarchicalInstancedStaticMeshComponent Object Reference") (`2D Movement Vector` :type "Vector2D Structure"))
  (bind _returnvalue (`SceneComponent.K2_GetComponentToWorld` HISMC))
  (`SceneComponent.K2_SetWorldTransform` HISMC (`KismetMathLibrary.MakeTransform` (`KismetMathLibrary.MakeVector` (+ (.x (.location _returnvalue)) `2D Movement Vector_X`) (+ `2D Movement Vector_Y` (.y (.location _returnvalue))) (.z (.location _returnvalue))) (.rotation _returnvalue) (.scale _returnvalue)) false false))

(fn `Move HISM Components`
  (params (`Movement Speed` :type "Float (double-precision)"))
  (`self.Move HISM Component In Axis` (`self.X- Axis Cars`) (`KismetMathLibrary.MakeVector2D` (* `Movement Speed` -1.0)))
  (`self.Move HISM Component In Axis` (`self.X+ Axis Cars`) (`KismetMathLibrary.MakeVector2D` `Movement Speed`))
  (`self.Move HISM Component In Axis` (`self.Y- Axis Cars`) (`KismetMathLibrary.MakeVector2D` 0.0 (* `Movement Speed` -1.0)))
  (`self.Move HISM Component In Axis` (`self.Y+ Axis Cars`) (`KismetMathLibrary.MakeVector2D` 0.0 `Movement Speed`)))

(fn `Spawn Car`
  (params (`HSMI Component` :type "HierarchicalInstancedStaticMeshComponent Object Reference") (IsX :type Boolean) (IsPositive :type Boolean) (Height :type "Float (double-precision)"))
  (bind _returnvalue (`KismetMathLibrary.Conv_BoolToDouble` IsX))
  (bind _motif_distance (`self.Motif Distance`))
  (bind _spawn_int_range (`self.Spawn Int Range`))
  (bind (_player_motif_point_location_x _player_motif_point_location_y) (break `IntPoint` (`self.Player Motif Point Location`)))
  (bind _random_postion_amount (`self.Random Postion Amount`))
  (bind _returnvalue_2 (* _spawn_int_range _motif_distance))
  (bind _returnvalue_3 (`KismetMathLibrary.Conv_BoolToDouble` (not IsX)))
  (bind _returnvalue_4 (* _player_motif_point_location_x _motif_distance))
  (bind _returnvalue_5 (* _player_motif_point_location_y _motif_distance))
  (bind _returnvalue_6 (`KismetMathLibrary.RandomFloatInRange` (* _random_postion_amount -1.0) _random_postion_amount))
  (bind _returnvalue_7 (- (* (`KismetMathLibrary.Conv_BoolToDouble` IsPositive) 2.0) 1.0))
  (bind _returnvalue_8 (* _returnvalue_7 -1.0))
  (bind _returnvalue_9 (* _returnvalue_7 (`self.Lane Adjacent Offset`)))
  (for _index (range (* _spawn_int_range -1) (+ _spawn_int_range 1))
    (bind _returnvalue_10 (* _index _motif_distance))
    (`InstancedStaticMeshComponent.AddInstanceWorldSpace` `HSMI Component` (`KismetMathLibrary.MakeTransform` (`KismetMathLibrary.MakeVector` (+ (* (+ _returnvalue_10 _returnvalue_4 _returnvalue_9) _returnvalue_3) (* (+ (+ (* _returnvalue_2 _returnvalue_8) _returnvalue_4) _returnvalue_6) _returnvalue)) (+ (* (+ _returnvalue_10 _returnvalue_5 _returnvalue_9) _returnvalue) (* (+ (+ (* _returnvalue_2 _returnvalue_8) _returnvalue_5) _returnvalue_6) _returnvalue_3)) Height) (`SceneComponent.K2_GetComponentRotation` `HSMI Component`)))))

(fn `Spawn Car Layers`
  (bind (_returnvalue_x _returnvalue_y _returnvalue_z) (`KismetMathLibrary.BreakVector` (`self.K2_GetActorLocation`)))
  (bind _lane_above_offset (`self.Lane Above Offset`))
  (for _index (range (`self.Layer Amount`))
    (bind _returnvalue (+ (* _index _lane_above_offset) _returnvalue_z))
    (`self.Spawn Car` (`self.X+ Axis Cars`) true true _returnvalue)
    (`self.Spawn Car` (`self.X- Axis Cars`) true false _returnvalue)
    (bind _returnvalue_2 (+ (* _lane_above_offset 0.5) _returnvalue))
    (`self.Spawn Car` (`self.Y+ Axis Cars`) false true _returnvalue_2)
    (`self.Spawn Car` (`self.Y- Axis Cars`) false false _returnvalue_2)))

(fn `UserConstructionScript`)